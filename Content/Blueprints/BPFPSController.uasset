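; First-person player controller for a battle royale game that sets up the ammo display and battle log on remote (non-authority) instances.
; At BeginPlay it creates both widgets, seeds the ammo count from the controlled character and binds to its ammo changes and the game state's player-joined event.
; AnnounceNewPlayer adds a timed "Joined" entry to the battle log, then calls BindNewPlayer to bind that player's death event.
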(event `self.ReceiveBeginPlay`
  (bind _controlledcharacter (`self.ControlledCharacter`))
  (`/Engine/EditorBlueprintResources/ActorMacros.Switch Has Authority`
    (:`Remote`
      (`|ExecutionSequence`
        (:`then_0`
          ;[1 1 1] Create ammo count display and bind change event
          (bind _returnvalue (`|CreateWidget` "/Game/Blueprints/UI/BPAmmoDisplay.BPAmmoDisplay_C" self))
          (set `self.AmmoDisplay` _returnvalue)
          (`UserWidget.AddToViewport` _returnvalue 0)
          (add `FPSCharacter.OnAmmoCountChanged` _controlledcharacter (`|CreateDelegate` _returnvalue :!event `Set Ammo`))
          ;[1 1 1] Set initial ammo count
          (bind _returnvalue_2 (`FPSCharacter.GetAmmoCount` _controlledcharacter))
          (`/Game/Blueprints/UI/BPAmmoDisplay.Set Ammo` _returnvalue _returnvalue_2))
        (:`then_1`
          ;[1 1 1] Battle log
          (bind _returnvalue_3 (`|CreateWidget` "/Game/Blueprints/UI/BP_BattleLog.BP_BattleLog_C" self))
          (bind _output_get (set `self.BattleLog` _returnvalue_3))
          (`UserWidget.AddToViewport` _output_get 0)
          ;[1 1 1] Bind new player event
          (bind _asbattle_royale_game_state (cast `BattleRoyaleGameState` (`GameplayStatics.GetGameState`)))
          (add `BattleRoyaleGameState.OnPlayerJoined` _asbattle_royale_game_state (`|CreateDelegate` self :!event `AnnounceNewPlayer`)))))))

(fn `AnnounceNewPlayer`
  (params (Player :type "FPSPlayerState Object Reference"))
  (bind _returnvalue (`|GenericCreateObject` "/Game/Blueprints/BPBattleLogEntryInfo.BPBattleLogEntryInfo_C" self))
  (set `BattleLogEntryInfo.ActionType` "Joined" _returnvalue)
  (set `BattleLogEntryInfo.Entry1` (`PlayerState.GetPlayerName` Player) _returnvalue)
  (set `BattleLogEntryInfo.TimeToLive` 10.0 _returnvalue)
  (`/Game/Blueprints/UI/BP_BattleLog.Add Entry` (`self.BattleLog`) _returnvalue)
  (`self.BindNewPlayer` Player))

(fn `BindNewPlayer`
  (params (Player :type "FPSPlayerState Object Reference"))
  (add `FPSPlayerState.OnPlayerDied` Player (`|CreateDelegate` (`self.BattleLog`) :!event `Add Entry`)))

(fn `UserConstructionScript`)